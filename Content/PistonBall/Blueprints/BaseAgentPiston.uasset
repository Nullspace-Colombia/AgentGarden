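; Base piston agent for the PistonBall game, exposing step, state, reward, done and reset functions in a reinforcement-learning style.
; Step counts frames and slides Body vertically to the height given by its indexed entry in the action array.
; State is Body's relative height, and reward depends on whether Ball's X is beyond the piston's.
; An episode ends when the counter reaches MaxFrames, and Reset reuses the same actor.
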(event `/unray/Blueprints/BI_Agent.Step`
  (params (Action :type "Array of Float (double-precision) (by ref)"))
  (bind _body (`self.Body`))
  (bind _counter (`self.Counter`))
  (bind (_relativelocation_x _relativelocation_y) (`KismetMathLibrary.BreakVector` (`SceneComponent.RelativeLocation` _body)))
  (`/Engine/EditorBlueprintResources/StandardMacros.IncrementInt` _counter
    (:`  `
      (`KismetSystemLibrary.PrintString` (`KismetStringLibrary.Conv_IntToString` _counter))
      (`KismetSystemLibrary.MoveComponentTo` _body (`KismetMathLibrary.MakeVector` _relativelocation_x _relativelocation_y (* (`|GetArrayItem` Action (`self.action`)) 100.0)) (struct) false false 0.08))))

(event `/unray/Blueprints/BI_Agent.SetActionID`
  (params (ActionID :type Integer))
  (set `self.action` ActionID))

(fn `GetID`
  (returns (ID :type Integer))
  (return 0))

(fn `GetReward`
  (returns (Reward :type "Float (double-precision)"))
  (bind _returnvalue_x (`KismetMathLibrary.BreakVector` (`self.K2_GetActorLocation`)))
  (bind _returnvalue_x_2 (`KismetMathLibrary.BreakVector` (`self.K2_GetActorLocation` (`self.ball`))))
  (`/Engine/EditorBlueprintResources/StandardMacros.CompareFloat` _returnvalue_x_2 _returnvalue_x
    (:`>`
      (set `self.reward` 0.5))
    (:`==`
      (set `self.reward` -0.5 :!label _label))
    (:`<`
      (goto _label)))
  (return (`self.reward`)))

(fn `GetSelfActor`
  (returns (Actor :type "Actor Object Reference"))
  (return self))

(fn `GetState`
  (returns (Observations :type "Array of Float (double-precision)"))
  (bind (_relativelocation_x _relativelocation_y _relativelocation_z) (`KismetMathLibrary.BreakVector` (`SceneComponent.RelativeLocation` (`self.Body`))))
  (return (`|MakeArray` _relativelocation_z)))

(fn `IsDone`
  (returns (bDone :type Boolean))
  (`/Engine/EditorBlueprintResources/StandardMacros.CompareInt` (`self.Counter`) (`self.max_frames`)
    (:`>`
      (set `self.Done` true :!label _label)
      (set `self.Counter` 0))
    (:`==`
      (goto _label))
    (:`<`
      (set `self.Done` false)))
  (return (`self.Done`)))

(fn `Reset`
  (returns (NewActor :type "/unray/Blueprints/BI_Agent Interface") (bCreateActor :type Boolean))
  (bind _body (`self.Body`))
  (bind (_relativelocation_x _relativelocation_y) (`KismetMathLibrary.BreakVector` (`SceneComponent.RelativeLocation` _body)))
  (`SceneComponent.K2_SetRelativeLocation` _body (`KismetMathLibrary.MakeVector` _relativelocation_x _relativelocation_y) false false)
  (return self false))

(fn `UserConstructionScript`)