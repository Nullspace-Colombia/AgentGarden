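; BP_Agent2 is the second agent in a step/reward/reset setup, inheriting stepping, state, reward and done logic from its parent.
; BeginPlay skips the parent's version and caches the carry box, then BP_Agent1 if that box exists.
; Reset spawns and returns a replacement at randomized X and fixed Y, relinks BP_Agent1 to it and clears episode variables on itself.
; Releasing G manually steps the other agent with a fixed action.
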(event `self.ReceiveBeginPlay`
  (bind _returnvalue (`GameplayStatics.GetActorOfClass` "/Game/Football/Blueprints/Agent1/BP_Ag_Prop_Box1.BP_Ag_Prop_Box1_C"))
  (`/Engine/EditorBlueprintResources/StandardMacros.IsValid` _returnvalue
    (:`Is Valid`
      (set `self.CarryBox` _returnvalue)
      (bind _returnvalue_2 (`GameplayStatics.GetActorOfClass` "/Game/Football/Blueprints/Agent1/BP_Agent1.BP_Agent1_C"))
      (set `self.Other agent` _returnvalue_2))))

(event `/unray/Blueprints/BI_Agent.SetID`
  (params (ID :type Integer))
  (`parent.SetID` ID))

(event `Key|G`
  (params (Key :type "Key Structure"))
  (:`Released`
    (`/unray/Blueprints/BI_Agent.Step` (`self.Other agent`) (`|MakeArray` 5.0))))

(event `/unray/Blueprints/BI_Agent.SetActionID`
  (params (ActionID :type Integer))
  (`parent.SetActionID` ActionID))

(event `/unray/Blueprints/BI_Agent.Step`
  (params (Action :type "Array of Float (double-precision) (by ref)"))
  (`parent.Step` Action))

(fn `GetID`
  (returns (ID :type Integer))
  (return (`self.ID`)))

(fn `GetReward`
  (returns (Reward :type "Float (double-precision)"))
  (bind _reward (`parent.GetReward`))
  (return _reward))

(fn `GetSelfActor`
  (returns (Actor :type "Actor Object Reference"))
  (bind _actor (`parent.GetSelfActor`))
  (return _actor))

(fn `GetState`
  (returns (Observations :type "Array of Float (double-precision)"))
  (bind _observations (`parent.GetState`))
  (return _observations))

(fn `IsDone`
  (returns (bDone :type Boolean))
  (bind _bdone (`parent.IsDone`))
  (return _bdone))

(fn `Reset`
  (returns (NewActor :type "/unray/Blueprints/BI_Agent Interface") (bCreateActor :type Boolean))
  (set `self.counter` 0)
  (bind _output_get (set `self.actor initial position` -850.0))
  (bind _returnvalue (`|SpawnActorFromClass` "BP_Agent2_C" (`KismetMathLibrary.MakeTransform` (`KismetMathLibrary.MakeVector` (`KismetMathLibrary.RandomFloatInRange` 50.0 210.0) _output_get 100.0) (struct :`Yaw` 90.0)) "AlwaysSpawn" "MultiplyWithRoot" null null))
  (bind _returnvalue_2 (`GameplayStatics.GetActorOfClass` "/Game/Football/Blueprints/Agent1/BP_Agent1.BP_Agent1_C"))
  (set `self.Other agent` _returnvalue_2)
  (set `/Game/Football/Blueprints/Agent1/BP_Agent1.Other agent` _returnvalue (`self.Other agent`))
  (set `self.done` false)
  (`KismetSystemLibrary.PrintString` "reset" false false)
  (set `self.Reward` 0.0)
  (set `self.max_y` (`self.actor initial position`))
  (return _returnvalue true))

(fn `UserConstructionScript`
  (`parent.UserConstructionScript`))