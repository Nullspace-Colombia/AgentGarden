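; Player character for a football game, built as a learning agent that is driven through Step actions or keyboard input.
; Each tick it moves, turns and fills an observation array with distance and tag-based type from fifteen arrow line traces.
; GetState, GetReward, IsDone and Reset expose the training loop, with reward from ball and goal proximity, a step penalty and a goal bonus.
; Box-carry, push and world-direction movement logic is leftover, unwired code.
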(event `self.ReceiveTick`
  (params (DeltaSeconds :type "Float (single-precision)"))
  (`self.Move`)
  (`self.Turn`)
  (`self.Trace`))

(event `EnhancedInput|/Game/Football/Inputs/IA_MoveDown`
  (params (ActionValue :type Boolean) (ElapsedSeconds :type "Float (double-precision)") (TriggeredSeconds :type "Float (double-precision)") (InputAction :type "InputAction Object Reference" :default "/Game/Football/Inputs/IA_MoveDown.IA_MoveDown")))

(event `EnhancedInput|/Game/Football/Inputs/IA_MoveLeft`
  (params (ActionValue :type Boolean) (ElapsedSeconds :type "Float (double-precision)") (TriggeredSeconds :type "Float (double-precision)") (InputAction :type "InputAction Object Reference" :default "/Game/Football/Inputs/IA_MoveLeft.IA_MoveLeft"))
  (:`Started`
    (set `self.Side` 0))
  (:`Completed`
    (set `self.Side` 1)))

(event `Move`
  (`self.AddMovementInput` (`self.GetActorForwardVector`) (`self.Forward`)))

(event `EnhancedInput|/Game/Football/Inputs/IA_MoveRight`
  (params (ActionValue :type Boolean) (ElapsedSeconds :type "Float (double-precision)") (TriggeredSeconds :type "Float (double-precision)") (InputAction :type "InputAction Object Reference" :default "/Game/Football/Inputs/IA_MoveRight.IA_MoveRight"))
  (:`Started`
    (set `self.Side` 2))
  (:`Completed`
    (set `self.Side` 1)))

(event `Turn`
  (`self.AddControllerYawInput` (select `int` (`self.Side`) :`0` -1.0 :`1` 0.0 :`2` 1.0 :!type "Float (single-precision)")))

(event `EnhancedInput|/Game/Football/Inputs/IA_MoveUp`
  (params (ActionValue :type Boolean) (ElapsedSeconds :type "Float (double-precision)") (TriggeredSeconds :type "Float (double-precision)") (InputAction :type "InputAction Object Reference" :default "/Game/Football/Inputs/IA_MoveUp.IA_MoveUp"))
  (:`Started`
    (set `self.Forward` 1.0)
    (set `self.Walk` true))
  (:`Completed`
    (set `self.Forward` 0.0)
    (set `self.Walk` false)))

(event `Trace`
  (for (_array_element _array_index) (`|MakeArray` (`self.Arrow1`) (`self.Arrow2`) (`self.Arrow3`) (`self.Arrow4`) (`self.Arrow5`) (`self.Arrow6`) (`self.Arrow7`) (`self.Arrow8`) (`self.Arrow9`) (`self.Arrow10`) (`self.Arrow11`) (`self.Arrow12`) (`self.Arrow13`) (`self.Arrow14`) (`self.Arrow15`))
    (bind (_distance _type) (`self.TraceArrow` _array_element 600.0))
    (`KismetArrayLibrary.Array_Set` (`self.obs`) _array_index _distance)
    (`KismetArrayLibrary.Array_Set` (`self.obs`) (+ _array_index 15) _type)))

(event `/unray/Blueprints/BI_Agent.Step`
  (params (Action :type "Array of Float (double-precision) (by ref)"))
  (set `self.Forward` (`|GetArrayItem` Action))
  (set `self.Side` (`KismetMathLibrary.FTrunc` (`|GetArrayItem` Action 1))))

(event `CheckJump`
  ;[0.9019 1 0.377] Check jump
  (if (`|EnumEquality` (`CharacterMovementComponent.MovementMode` (`self.CharacterMovement`)) "MOVE_Falling")
    (set `self.Jumping` true)
    (else
      (set `self.Jumping` false))))

(event `CheckPush`
  ;[0.9004 1 0.2708] Check Push
  (if (or (`self.Push`) (`self.bCarry`))
    (set `CharacterMovementComponent.MaxWalkSpeed` 250.0 (`self.CharacterMovement`))
    (else
      (set `CharacterMovementComponent.MaxWalkSpeed` 500.0 (`self.CharacterMovement`)))))

(event `self.ReceiveBeginPlay`
  (`|ExecutionSequence`
    (:`then_0`
      (bind _asplayer_controller (cast `PlayerController` (`self.GetController`)))
      (bind _returnvalue (pcsubsystem `EnhancedInputLocalPlayerSubsystem` _asplayer_controller))
      (`/Engine/EditorBlueprintResources/StandardMacros.IsValid` _returnvalue
        (:`Is Valid`
          (`EnhancedInputSubsystemInterface.AddMappingContext` _returnvalue "/Game/Football/Inputs/IMC_Agent.IMC_Agent" 0 (struct)))))
    (:`then_1`
      (bind _returnvalue_2 (`GameplayStatics.GetActorOfClass` "/Game/Football/Blueprints/Agent1/BP_Agent2.BP_Agent2_C"))
      (set `self.Other agent` _returnvalue_2))
    (:`then_2`
      (bind _returnvalue_3 (`GameplayStatics.GetActorOfClass` "/Game/Football/Blueprints/Agent1/BP_Ag_Prop_Box1.BP_Ag_Prop_Box1_C"))
      (`/Engine/EditorBlueprintResources/StandardMacros.IsValid` _returnvalue_3
        (:`Is Valid`
          (set `self.CarryBox` _returnvalue_3))))))

(event `Key|C`
  (params (Key :type "Key Structure"))
  (:`Pressed`
    (`/Engine/EditorBlueprintResources/StandardMacros.IsValid` (`self.Shield`)
      (:`Is Valid`
        (if (`self.bCarry`)
          (`self.K2_DetachFromActor` (`self.Shield`) "KeepWorld" "KeepWorld" "KeepWorld")
          (set `self.bCarry` false)
          (else
            (`/Game/Football/Blueprints/Agent1/BP_Shield.ChangeCollision` (`self.Shield`))
            (`self.K2_AttachToComponent` (`self.Shield`) (`self.Mesh`) "hand_LSocket" "SnapToTarget" "SnapToTarget" "KeepWorld" true)
            (set `self.bCarry` true)))))))

(event `AlwaysMove`
  (`self.AddMovementInput` (`self.World Direction Vector`) 0.5)
  (if (> (`KismetMathLibrary.VSize` (`MovementComponent.Velocity` (`self.CharacterMovement`))) 0.0)
    (set `self.Walk` true)
    (else
      (set `self.Walk` false))))

(event `EnhancedInput|/Game/Football/Inputs/IA_Jump`
  (params (ActionValue :type Boolean) (ElapsedSeconds :type "Float (double-precision)") (TriggeredSeconds :type "Float (double-precision)") (InputAction :type "InputAction Object Reference" :default "/Game/Football/Inputs/IA_Jump.IA_Jump")))

(event `EnhancedInput|/Game/Football/Inputs/IA_Grab`
  (params (ActionValue :type Boolean) (ElapsedSeconds :type "Float (double-precision)") (TriggeredSeconds :type "Float (double-precision)") (InputAction :type "InputAction Object Reference" :default "/Game/Football/Inputs/IA_Grab.IA_Grab")))

(event `self.Box.OnComponentBeginOverlap`
  (params (OverlappedComponent :type "PrimitiveComponent Object Reference") (OtherActor :type "Actor Object Reference") (OtherComp :type "PrimitiveComponent Object Reference") (OtherBodyIndex :type Integer) (bFromSweep :type Boolean) (SweepResult :type "HitResult Structure (by ref)")))

(event `self.Box.OnComponentEndOverlap`
  (params (OverlappedComponent :type "PrimitiveComponent Object Reference") (OtherActor :type "Actor Object Reference") (OtherComp :type "PrimitiveComponent Object Reference") (OtherBodyIndex :type Integer)))

(event `/unray/Blueprints/BI_Agent.SetActionID`
  (params (ActionID :type Integer))
  (set `self.Action ID` ActionID))

(event `/unray/Blueprints/BI_Agent.SetID`
  (params (ID :type Integer))
  (set `self.ID` ID))

(fn `GetID`
  (returns (ID :type Integer))
  (return (`self.ID`)))

(fn `GetReward`
  (returns (Reward :type "Float (double-precision)"))
  (bind _ball (`self.ball`))
  (bind _returnvalue (`SceneComponent.K2_GetComponentLocation` (`/Game/Football/Blueprints/BP_BALL.Sphere` _ball)))
  (bind _outactors (`GameplayStatics.GetAllActorsWithTag` "goal"))
  (bind _output_get (set `self.Reward` (+ (`self.Reward`) (/ 1.0 (`KismetMathLibrary.Vector_Distance` (`self.K2_GetActorLocation`) _returnvalue)) (/ 1.0 (`KismetMathLibrary.Vector_Distance` _returnvalue (`self.K2_GetActorLocation` (`|GetArrayItem` _outactors)))) -0.005 (select `bool` (`/Game/Football/Blueprints/BP_BALL.gol` _ball) :`true` 20.0))))
  (return _output_get))

(fn `GetSelfActor`
  (returns (Actor :type "Actor Object Reference"))
  (return self))

(fn `GetState`
  (returns (Observations :type "Array of Float (double-precision)"))
  (locals (NewLocalVar :type "EDrawDebugTrace Enum" :default "None"))
  (return (`self.obs`)))

(fn `IsDone`
  (returns (bDone :type Boolean))
  (bind _outactors (`GameplayStatics.GetAllActorsOfClass` "/Game/Football/Blueprints/BP_BALL.BP_BALL_C"))
  (return (`/Game/Football/Blueprints/BP_BALL.gol` (`|GetArrayItem` _outactors))))

(fn `Reset`
  (returns (NewActor :type "/unray/Blueprints/BI_Agent Interface") (bCreateActor :type Boolean))
  (`self.K2_SetActorLocation` (-11290.805484 -830.706902 384.524756))
  (bind _outactors (`GameplayStatics.GetAllActorsOfClass` "/Game/Football/Blueprints/BP_BALL.BP_BALL_C"))
  (`/Game/Football/Blueprints/BP_BALL.ResetBall` (`|GetArrayItem` _outactors))
  (return null false))

(fn `TraceArrow`
  (params (Arrow :type "ArrowComponent Object Reference") (Lenght :type "Float (single-precision)"))
  (returns (Distance :type "Float (double-precision)") (Type :type "Float (double-precision)"))
  (locals (Type1 :type "Float (double-precision)"))
  (bind _returnvalue (`SceneComponent.K2_GetComponentLocation` Arrow))
  (bind (_outhit _returnvalue_2) (`KismetSystemLibrary.LineTraceSingle` :`Start` _returnvalue :`End` (+ _returnvalue (* (`SceneComponent.GetForwardVector` Arrow) Lenght)) :`TraceChannel` "TraceTypeQuery1" :`DrawDebugType` "ForOneFrame" :`TraceColor` (struct :`R` 1.0 :`G` 0.758232 :`A` 1.0)))
  (if _returnvalue_2
    (bind (_bblockinghit _binitialoverlap _time _distance _location _impactpoint _normal _impactnormal _physmat _hitactor) (`GameplayStatics.BreakHitResult` _outhit))
    (`KismetSystemLibrary.PrintString` "pared" (`self.ActorHasTag` _hitactor "pared"))
    (switch `name` (`|GetArrayItem` (`Actor.Tags` _hitactor))
      (:`Default`
        (set `local.Type1` 0.0))
      (:`wall`
        (set `local.Type1` 1.0))
      (:`ball`
        (set `local.Type1` 2.0))
      (:`opponent`
        (set `local.Type1` 3.0))
      (:`goal`
        (set `local.Type1` 4.0))))
  (return _distance (`local.Type1`)))

(fn `UserConstructionScript`)