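; BP_Ag_Prop_Box1 is a physics box prop in the Football level, tied to BP_Agent1.
; On BeginPlay it caches the BP_Agent1 actor, then its Box component's overlap events maintain a flag for whether that agent is overlapping it.
; Tick watches for the box falling below the floor, then teleports it to a fixed position and resets BlueBox's angular and linear velocity.
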(event `self.ReceiveTick`
  (params (DeltaSeconds :type "Float (single-precision)"))
  (bind (_returnvalue_x _returnvalue_y _returnvalue_z) (`KismetMathLibrary.BreakVector` (`self.K2_GetActorLocation`)))
  (if (<= _returnvalue_z -100.0)
    (`self.K2_SetActorLocation` (50.0 450.0 0.0) false true)
    (`PrimitiveComponent.SetAllPhysicsAngularVelocityInDegrees` (`self.BlueBox`) (0.0 0.0 0.0) false)
    (`PrimitiveComponent.SetAllPhysicsLinearVelocity` (`self.BlueBox`) (0.0 0.0 0.0) false)))

(event `self.ReceiveBeginPlay`
  (bind _returnvalue (`GameplayStatics.GetActorOfClass` "/Game/Football/Blueprints/Agent1/BP_Agent1.BP_Agent1_C"))
  (set `self.actor1` _returnvalue))

(event `self.Box.OnComponentBeginOverlap`
  (params (OverlappedComponent :type "PrimitiveComponent Object Reference") (OtherActor :type "Actor Object Reference") (OtherComp :type "PrimitiveComponent Object Reference") (OtherBodyIndex :type Integer) (bFromSweep :type Boolean) (SweepResult :type "HitResult Structure (by ref)"))
  (if (== OtherActor (`self.actor1`))
    (set `self.IsOverlapping_actor1` true)))

(event `self.Box.OnComponentEndOverlap`
  (params (OverlappedComponent :type "PrimitiveComponent Object Reference") (OtherActor :type "Actor Object Reference") (OtherComp :type "PrimitiveComponent Object Reference") (OtherBodyIndex :type Integer))
  (if (== OtherActor (`self.actor1`))
    (set `self.IsOverlapping_actor1` false)))

(fn `UserConstructionScript`)