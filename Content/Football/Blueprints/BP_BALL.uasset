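; BP_BALL is the football actor, which detects goals and can reset itself for another attempt.
; Its Sphere sets the Gol flag and prints "goal" when it begins overlapping an actor tagged "goal".
; ResetBall clears Gol, moves both actor and Sphere to separately randomized XY offsets around NewLocation, and zeroes the Sphere's linear physics velocity.
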(event `self.Sphere.OnComponentBeginOverlap`
  (params (OverlappedComponent :type "PrimitiveComponent Object Reference") (OtherActor :type "Actor Object Reference") (OtherComp :type "PrimitiveComponent Object Reference") (OtherBodyIndex :type Integer) (bFromSweep :type Boolean) (SweepResult :type "HitResult Structure (by ref)"))
  (if (`self.ActorHasTag` OtherActor "goal")
    (set `self.gol` true)
    (`KismetSystemLibrary.PrintString` "goal" true true (struct :`R` 1.0 :`G` 0.052541 :`B` 0.283838 :`A` 1.0))))

(event `ResetBall`
  (bind _returnvalue (+ (`self.New Location`) (`KismetMathLibrary.MakeVector` (`KismetMathLibrary.RandomFloatInRange` -600.0 600.0) (`KismetMathLibrary.RandomFloatInRange` -800.0 800.0))))
  (`self.K2_SetActorLocation` _returnvalue)
  (set `self.gol` false)
  (`SceneComponent.K2_SetWorldLocation` (`self.Sphere`) _returnvalue false false)
  (`PrimitiveComponent.SetPhysicsLinearVelocity` (`self.Sphere`) (0.0 0.0 0.0) false "None"))

(fn `UserConstructionScript`)