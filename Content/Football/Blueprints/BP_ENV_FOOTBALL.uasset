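; Football environment actor that assembles a ball, an agent and a connector from its child actor components.
; On BeginPlay it attaches the ball and agent to its root at fixed relative offsets and stores each resulting world position in that actor's NewLocation.
; It gives the agent a reference to the ball, saves it as Agent and registers the Connector_SA child through SetConnector.
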(event `self.ReceiveBeginPlay`
  (bind _asbp_ball (cast `/Game/Football/Blueprints/BP_BALL` (`ChildActorComponent.ChildActor` (`self.BP_BALL`))))
  (`SceneComponent.K2_AttachToComponent` (`Actor.RootComponent` _asbp_ball) (`self.DefaultSceneRoot`) "None" "KeepRelative" "KeepRelative" "KeepRelative" true)
  (`self.K2_SetActorRelativeLocation` _asbp_ball (30.0 -60.0 50.0) false false)
  (set `/Game/Football/Blueprints/BP_BALL.New Location` (`self.K2_GetActorLocation` _asbp_ball) _asbp_ball)
  (bind _asbp_agent_p (cast `/Game/Football/Blueprints/Agent1/BP_AgentP` (`ChildActorComponent.ChildActor` (`self.BP_AgentP`)))
    (:`then`
      (`SceneComponent.K2_AttachToComponent` (`Actor.RootComponent` _asbp_agent_p) (`self.DefaultSceneRoot`) "None" "KeepRelative" "KeepRelative" "KeepRelative" true)
      (`self.K2_SetActorRelativeLocation` _asbp_agent_p (20.0 -240.0 110.0) false false)
      (set `/Game/Football/Blueprints/Agent1/BP_AgentP.NewLocation` (`self.K2_GetActorLocation` _asbp_agent_p) _asbp_agent_p)
      (set `/Game/Football/Blueprints/Agent1/BP_AgentP.ball` _asbp_ball _asbp_agent_p)
      (set `self.Agent` _asbp_agent_p)
      (bind _asconnector_sa (cast `/unray/Blueprints/Connector_SA` (`ChildActorComponent.ChildActor` (`self.Connector_SA`))))
      (`self.SetConnector` _asconnector_sa))
    (:`CastFailed`
      (`KismetSystemLibrary.PrintString` "Hello"))))

(fn `UserConstructionScript`)