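; NPC environment actor that pairs an NPC agent with a Connector_SA, both hosted through child actor components.
; On BeginPlay it casts the NPC child actor to BP_NPC_C and stores it as Agent, then casts the connector child and passes it to SetConnector.
; Either failed cast halts the setup, and Tick, overlap and construction add no logic of their own.
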(event `self.ReceiveBeginPlay`
  (bind _asbp_npc_c (cast `/Game/NPC/Blueprints/BP_NPC_C` (`ChildActorComponent.ChildActor` (`self.BP_NPC_C`))))
  (set `self.Agent` _asbp_npc_c)
  (bind _asconnector_sa (cast `/unray/Blueprints/Connector_SA` (`ChildActorComponent.ChildActor` (`self.Connector_SA`))))
  (`self.SetConnector` _asconnector_sa))

(fn `UserConstructionScript`
  (`parent.UserConstructionScript`))